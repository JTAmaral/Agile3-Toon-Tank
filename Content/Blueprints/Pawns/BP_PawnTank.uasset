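; BP_PawnTank is the tank pawn Blueprint that handles taking damage and losing the game.
; On BeginPlay it creates and displays a health bar widget.
; Any damage removes a fixed amount from the shield while it is active, switching it off when depleted, otherwise from health.
; At zero health it destroys the player's tank pawn and shows the game-end widget.
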(event EventBeginPlay
  (bind _returnvalue (UserInterface|CreateWidget "/Game/Blueprints/Widgets/WBP_HealthBar.WBP_HealthBar_C"))
  (bind _output_get (Variables|Default|SetHealthBarReference _returnvalue))
  (UserInterface|Viewport|AddtoViewport _output_get 0))

(event Collision|EventActorBeginOverlap
  (params (OtherActor :type Actor%20Object%20Reference)))

(event EventTick
  (params (DeltaSeconds :type Float%20%28single-precision%29)))

(event Game|Damage|EventAnyDamage
  (params (Damage :type Float%20%28single-precision%29) (DamageType :type Damage%20Type%20Object%20Reference) (InstigatedBy :type Controller%20Object%20Reference) (DamageCauser :type Actor%20Object%20Reference))
  (if (Variables|Default|GetisShieldActivated)
    (Variables|Default|SetCurrentShieldHealth (- (Variables|Default|GetCurrentShieldHealth) 1e+01))
    (if (<= (Variables|Default|GetCurrentShieldHealth) 0.0)
      (Variables|Default|SetisShieldActivated false))
    (else
      (Variables|Default|SetCurrentHealth (- (Variables|Default|GetCurrentHealth) 1e+01))
      (if (<= (Variables|Default|GetCurrentHealth) 0.0)
        (bind _asbp_pawn_tank (Utilities|Casting|CastToBP_PawnTank (Game|Player|GetPlayerPawn 0)))
        (Actor|DestroyActor _asbp_pawn_tank)
        (bind _returnvalue (UserInterface|CreateWidget "/Game/Blueprints/Widgets/WBP_GameEnd.WBP_GameEnd_C"))
        (UserInterface|Viewport|AddtoViewport _returnvalue 0)))))

(fn ConstructionScript)